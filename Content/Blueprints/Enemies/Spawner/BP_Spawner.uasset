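; Enemy spawner that spawns an initial wave of BP_Enemy AI pawns on BeginPlay and has an OnDieEnemy event that spawns more.
; SpawnEnemies shuffles the spawn point list, then cycles a wrapping index through it to place each pawn.
; Its loop runs while the counter is at least zero, so it attempts one spawn more than requested.
; Each spawned enemy's death dispatcher gets an event bound to it.
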(event Custom|OnDieEnemy
  (CallFunction|SpawnEnemies 2))

(event EventBeginPlay
  (CallFunction|SpawnEnemies 3))

(fn ConstructionScript)

(fn SpawnEnemies
  (params (EnemuesCount :type Integer))
  (LocalVariables|SetEnemiesToSpawn EnemuesCount)
  (Utilities|Array|Shuffle (Variables|Default|GetSpawnPoints))
  (while (>= (LocalVariables|GetEnemiesToSpawn) 0)
    (Math|Integer|DecrementInt (LocalVariables|GetEnemiesToSpawn)
      (:%20%20
        (bind _result (Math|Integer|IncrementInt (LocalVariables|GetIndex))
          (:%20%20
            (LocalVariables|SetIndex (Math|Integer|%(Integer) _result (Utilities|Array|Length (Variables|Default|GetSpawnPoints))))
            (bind _returnvalue (AI|SpawnAIFromClass "/Game/Blueprints/Enemies/BP_Enemy.BP_Enemy_C" 0 (Transformation|GetActorLocation (Utilities|Array|Get(acopy) (Variables|Default|GetSpawnPoints) (LocalVariables|GetIndex))) "0, 0, 0" false 0))
            (bind _asbp_enemy (Utilities|Casting|CastToBP_Enemy _returnvalue))
            (EventDispatchers|BindEventtoEDonDie _asbp_enemy (EventDispatchers|CreateEvent :!event Custom|OnDieEnemy))))))))