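; Enemy that chases the player's BP_BaseCharacter via AI MoveTo and damages any BP_BaseCharacter entering its sphere.
; The chase starts on BeginPlay and is reissued after non-lethal hits and on PawnSensing sightings, which also set walk speed.
; Incoming damage is treated as a fraction of MaxHealth, and the actor destroys itself at zero health or below.
; Destruction fires the OnDie event dispatcher.
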(event OnComponentBeginOverlap(Sphere)
  (params (OverlappedComponent :type Primitive%20Component%20Object%20Reference) (OtherActor :type Actor%20Object%20Reference) (OtherComp :type Primitive%20Component%20Object%20Reference) (OtherBodyIndex :type Integer) (bFromSweep :type Boolean) (SweepResult :type Hit%20Result%20Structure%20%28by%20ref%29))
  (bind _asbp_base_character (Utilities|Casting|CastToBP_BaseCharacter OtherActor))
  (Game|Damage|ApplyDamage _asbp_base_character (Variables|Constants|GetDamage) 0 0))

(event OnSeePawn(PawnSensing)
  (params (Pawn :type Pawn%20Object%20Reference))
  (Utilities|MovetoPlayer)
  (Variables|/Script/Engine.CharacterMovementComponent|SetMaxWalkSpeed (Variables|Character|GetCharacterMovement) 3e+02))

(event Custom|OnTakeAnyDamage_Event
  (params (DamagedActor :type Actor%20Object%20Reference) (Damage :type Float%20%28single-precision%29) (DamageType :type Damage%20Type%20Object%20Reference) (InstigatedBy :type Controller%20Object%20Reference) (DamageCauser :type Actor%20Object%20Reference))
  (Utilities|TakeDamage Damage)
  (if (<= (Variables|Default|GetCurrentHealth) 0.0)
    (Actor|DestroyActor)
    (else
      (Utilities|MovetoPlayer))))

(event EventBeginPlay
  (Utilities|MovetoPlayer)
  (EventDispatchers|BindEventtoOnTakeAnyDamage (delegate Custom|OnTakeAnyDamage_Event)))

(event EventDestroyed
  (Default|CallEDonDie))

(fn ConstructionScript)