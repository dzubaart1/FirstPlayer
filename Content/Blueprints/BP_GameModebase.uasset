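; Game mode base that handles player death by recording the best score and showing the game over screen.
; On BeginPlay it caches the player's BP_BaseCharacter and binds to its death-check dispatcher.
; When health is zero or below, it loads or creates a BP_SaveGame, saves the score only if it beats the stored best, then calls ShowGameOver on BP_GameInstance.
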(event Custom|CheckDeathEvent_Event
  (if (<= (Variables|/Game/Blueprints/Character/BP_BaseCharacter.BP_BaseCharacter_C|GetCurrentHealth (Variables|Default|GetBaseCharacter)) 0.0)
    (CallFunction|SaveScoreAmount (Variables|/Game/Blueprints/Character/BP_BaseCharacter.BP_BaseCharacter_C|GetCurrentScore (Variables|Default|GetBaseCharacter)))
    (bind _asbp_game_instance (Utilities|Casting|CastToBP_GameInstance (Game|GetGameInstance)))
    (Default|ShowGameOver _asbp_game_instance)))

(event EventBeginPlay
  (bind _asbp_base_character (Utilities|Casting|CastToBP_BaseCharacter (Game|GetPlayerCharacter 0)))
  (bind _output_get (Variables|Default|SetBaseCharacter _asbp_base_character))
  (EventDispatchers|BindEventtoEDCheckDeath _output_get (delegate Custom|CheckDeathEvent_Event)))

(fn ConstructionScript)

(fn SaveScoreAmount
  (params (ScoreAmount :type Integer))
  (Variables|Default|SetCurrentScore ScoreAmount)
  (bind _returnvalue (SaveGame|DoesSaveGameExist (Variables|Default|GetSlot%20Name)))
  (if _returnvalue
    (bind _returnvalue_2 (SaveGame|LoadGamefromSlot (Variables|Default|GetSlot%20Name)))
    (Variables|Default|SetSaveGame _returnvalue_2)
    (else
      (bind _returnvalue_3 (SaveGame|CreateSaveGameObject "/Game/Blueprints/BP_SaveGame.BP_SaveGame_C"))
      (bind _output_get (Variables|Default|SetSaveGame _returnvalue_3))))
  (bind _asbp_save_game (Utilities|Casting|CastToBP_SaveGame _output_get))
  (if (> (Variables|Default|GetCurrentScore) (Variables|/Game/Blueprints/BP_SaveGame.BP_SaveGame_C|GetBestScore _asbp_save_game))
    (Variables|/Game/Blueprints/BP_SaveGame.BP_SaveGame_C|SetBestScore _asbp_save_game (Variables|Default|GetCurrentScore))
    (SaveGame|SaveGametoSlot (Variables|Default|GetSaveGame) (Variables|Default|GetSlot%20Name))))